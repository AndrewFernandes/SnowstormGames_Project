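; Player character for a stealth game: collect two tagged objectives to win, lose when Alert reaches 100.
; Hit events destroy tagged pickups, setting objective or power-up flags or restoring capped Energy.
; Held stealth drains Energy on Tick and locks when depleted; counters throttle that drain and slow the Alert gain from PlayerDetected.
; Winning or losing shows a GameOverScreen widget and pauses the game.
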(event `InputAxis|MoveForward`
  (params (AxisValue :type "Float (single-precision)"))
  (bind _speed (`self.Speed`))
  (`self.K2_AddActorWorldOffset` (`KismetMathLibrary.MakeVector` (* AxisValue _speed) (* _speed (stale `InputAxis|MoveRight` AxisValue))) :!label _label))

(event `InputAxis|MoveRight`
  (params (AxisValue :type "Float (single-precision)"))
  (goto _label))

(event `InputAction|Stealth`
  (params (Key :type "Key Structure"))
  (:`Pressed`
    (if (not (`self.StealthLock`))
      (set `self.Stealthed` true)
      (`KismetSystemLibrary.PrintString` "Stealth On")))
  (:`Released`
    (set `self.Stealthed` false)
    (`KismetSystemLibrary.PrintString` "Stelth Off")))

(event `self.ReceiveHit`
  (params (MyComp :type "PrimitiveComponent Object Reference") (Other :type "Actor Object Reference") (OtherComp :type "PrimitiveComponent Object Reference") (bSelfMoved :type Boolean) (HitLocation :type "Vector Structure") (HitNormal :type "Vector Structure") (NormalImpulse :type "Vector Structure") (Hit :type "HitResult Structure (by ref)"))
  (bind _energy (`self.Energy`))
  ;[1 1 1] Determines what player hit, deletes hit actor if necessary, and changes variables if necessary.
  (if (`self.ActorHasTag` Other "ObjOne")
    (`self.K2_DestroyActor` Other)
    (set `self.ObjectiveOneGot` true)
    ;[1 1 1] Winning
    (if (and (`self.ObjectiveOneGot`) (`self.ObjectiveTwoGot`)) :!label _label_2
      (bind _returnvalue (`|CreateWidget` "/Game/Custom_Blueprints/GameOverScreen.GameOverScreen_C" (`GameplayStatics.GetPlayerController` 0)))
      (set `/Game/Custom_Blueprints/GameOverScreen.isWon` true _returnvalue)
      (`UserWidget.AddToViewport` _returnvalue 0)
      (`GameplayStatics.SetGamePaused` true))
    (elif (`self.ActorHasTag` Other "objTwo")
      (`self.K2_DestroyActor` Other)
      (set `self.ObjectiveTwoGot` true)
      (goto _label_2)
      (elif (`self.ActorHasTag` Other "PowerUp")
        (`self.K2_DestroyActor` Other)
        (set `self.PowerUpGot` true)
        (elif (`self.ActorHasTag` Other "EnergyUp")
          (`self.K2_DestroyActor` Other)
          ;[1 1 1] Gaining energy from EnergyBoost, but doesn't go beyond 100.
          (if (<= _energy 75.0)
            (set `self.Energy` (+ _energy 25.0))
            (set `self.StealthLock` false)
            (else
              (set `self.Energy` 100.0)))
          (`KismetSystemLibrary.PrintString` (`KismetStringLibrary.Concat_StrStr` "Energy Now " (`KismetStringLibrary.Conv_DoubleToString` _energy)) true true (struct :`R` 0.074376 :`G` 1.0 :`A` 1.0)))))))

(event `self.ReceiveTick`
  (params (DeltaSeconds :type "Float (single-precision)"))
  (bind _energycounter (`self.EnergyCounter`))
  ;[1 1 1] Losing
  (if (>= (`self.Alert`) 100.0)
    (bind _returnvalue (`|CreateWidget` "/Game/Custom_Blueprints/GameOverScreen.GameOverScreen_C" (`GameplayStatics.GetPlayerController` 0)))
    (set `/Game/Custom_Blueprints/GameOverScreen.isWon` false _returnvalue)
    (`UserWidget.AddToViewport` _returnvalue 0)
    (`GameplayStatics.SetGamePaused` true)
    (elif (and (`self.Stealthed`) (> (`self.Energy`) 0.0))
      (bind _result (`/Engine/EditorBlueprintResources/StandardMacros.IncrementFloat` _energycounter)
        (:`  `
          (if (== _result 1.0)
            (bind _result_2 (`/Engine/EditorBlueprintResources/StandardMacros.DecrementFloat` (`self.Energy`))
              (:`  `
                (`KismetSystemLibrary.PrintString` (`KismetStringLibrary.Concat_StrStr` "Energy is Now " (`KismetStringLibrary.Conv_DoubleToString` _result_2)))
                (if (== _result_2 0.0)
                  (set `self.Stealthed` false)
                  (set `self.StealthLock` true)
                  (`KismetSystemLibrary.PrintString` "Stealth Off"))))
            (elif (== _energycounter 6.0)
              (set `self.EnergyCounter` 0.0))))))))

(event `Player Detected`
  ;[1 1 1] Player gets detected by enemies.
  (if (`self.Stealthed`)
    (bind _result (`/Engine/EditorBlueprintResources/StandardMacros.IncrementFloat` (`self.StealthCounter`))
      (:`  `
        (if (== _result 1.0)
          (bind _result_2 (`/Engine/EditorBlueprintResources/StandardMacros.IncrementFloat` (`self.Alert`) :!label _label_3)
            (:`  `
              (`KismetSystemLibrary.PrintString` (`KismetStringLibrary.Concat_StrStr` "Alert is now at " (`KismetStringLibrary.Conv_DoubleToString` _result_2)))))
          (elif (== _result 4.0)
            (set `self.StealthCounter` 0.0)))))
    (else
      (goto _label_3))))

(fn `UserConstructionScript`)